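; Player stats component that holds a Stats struct with health, mana, stamina, experience, gold and a saved location.
; It exposes a stamina check that gates sprinting and a Sprinting function that subtracts a given amount from stamina, with no clamping.
; Tick calls a debug event that prints health, mana, stamina, experience and gold as red on-screen text every frame.
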(event `self.ReceiveTick`
  (params (DeltaSeconds :type "Float (single-precision)"))
  (`self.DebugStats` 0.0))

(event `DebugStats`
  (params (Duration :type "Float (double-precision)"))
  (bind (_health _mana _stamina _savedlocation _gold _experience) (break `/Game/Developer/Structures/S_Stats` (`self.Stats`)))
  (`KismetSystemLibrary.PrintText` (`|FormatText` "HP: {health}, MP: {mana}, Stam: {stamina}, XP: {experience}, Gold: {gold}" _health _mana _stamina _experience _gold) true true (struct :`R` 1.0 :`G` 0.008671 :`B` 0.013452 :`A` 1.0) Duration))

(fn `GetCanSprint`
  (returns (CanSprint :type Boolean))
  (bind (_stats_health _stats_mana _stats_stamina) (break `/Game/Developer/Structures/S_Stats` (`self.Stats`)))
  (return (> _stats_stamina 1.0)) ; Return true if stamina is greater than 1
)

(fn `Sprinting`
  (params (ReduceStaminaBy :type "Float (double-precision)" :default 2.0))
  (bind (_stats_health _stats_mana _stats_stamina _stats_savedlocation _stats_gold _stats_experience) (break `/Game/Developer/Structures/S_Stats` (`self.Stats`)))
  (set `self.Stats` (make `/Game/Developer/Structures/S_Stats` _stats_health _stats_mana (- _stats_stamina ReduceStaminaBy) _stats_savedlocation _stats_gold _stats_experience)))