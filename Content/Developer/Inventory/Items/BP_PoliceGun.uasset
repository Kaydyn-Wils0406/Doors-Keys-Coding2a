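; Police gun inventory item that the player can pick up and drop, with shooting and melee animations left unfinished.
; PickUp stores the owner, disables collision and returns the item type; Drop clears the held item, restores physics and applies a forward impulse.
; Use and AlternateUse are empty, leaving their timeline-driven shoot and gun-hit motions disconnected.
; BackToStart reverses the shoot motion, but its HasBeenUsed flag is set only in disconnected nodes.
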(event `self.ReceiveBeginPlay`
  (bind _asbp_custom_first_person_character (cast `/Game/Developer/BluePrints/BP_CustomFirstPersonCharacter` (`GameplayStatics.GetPlayerCharacter` 0)))
  (set `self.Player` _asbp_custom_first_person_character))

(event `/Game/Developer/Interaction/BPI_Item.Drop`
  (bind _policegun (`self.PoliceGun`))
  ; PickUp and Drop
  (set `/Game/Developer/Interaction/BPC_Interact.HeldItem` null (`self.Owner_0`))
  (`PrimitiveComponent.SetCollisionEnabled` _policegun "QueryAndPhysics")
  (`PrimitiveComponent.SetSimulatePhysics` _policegun true)
  (`PrimitiveComponent.AddImpulse` _policegun (* (`SceneComponent.GetForwardVector` _policegun) 500.0) "None" false))

(event `/Game/Developer/Interaction/BPI_Item.Use`
  ; Use - Shoot
)

(event `BackToStart`
  ; Use - Shoot
  (if (`self.bHasBeenUsed`)
    (set `self.bHasBeenUsed` false)
    (bind (_direction _shooting _aim) (`Timeline|Shoot` :!via `ReverseFromEnd`)
      (:`Update`
        (`SceneComponent.K2_SetRelativeLocationAndRotation` (`self.PoliceGun`) (`KismetMathLibrary.VLerp` (0.0 0.0 0.0) (0.0 -15.0 30.0) _aim) (`KismetMathLibrary.RLerp` (struct) (struct :`Pitch` 60.0) _shooting) false false)
        (`KismetSystemLibrary.Delay` 1.0)
        (`self.BackToStart`)))))

(event `/Game/Developer/Interaction/BPI_Item.AlternateUse`
  ; Alternate Use - Hit with Gun
)

(fn `NewFunction`)

(fn `PickUp`
  (params (Owner :type "/Game/Developer/Interaction/BPC_Interact Object Reference"))
  (returns (`Item Type` :type "/Game/Developer/BluePrints/E_item Enum"))
  (set `self.Owner_0` Owner)
  (`PrimitiveComponent.SetCollisionEnabled` (`self.PoliceGun`) "NoCollision")
  (return (`self.ItemType`)))

(fn `UserConstructionScript`)