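; BP_Key is an inventory key item that the player picks up, drops, or uses to open doors.
; PickUp stores the owner, plays a jingle, increments the player's key count, disables collision and registers itself with GM_SaveLoad's level state so it stays gone on reload.
; Drop re-enables physics and throws the key forward.
; Use briefly delays, line-traces forward for a BP_Doorrr, then drops, opens the door and destroys the key.
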(event `self.ReceiveBeginPlay`
  (bind _asbp_custom_first_person_character (cast `/Game/Developer/BluePrints/BP_CustomFirstPersonCharacter` (`GameplayStatics.GetPlayerCharacter` 0)))
  (set `self.CustomePlayer` _asbp_custom_first_person_character))

(event `/Game/Developer/Interaction/BPI_Item.Drop`
  (bind _key (`self.Key`))
  (set `/Game/Developer/BPC/BPC_Interact.HeldItem` null (`self.Owner_0`)) ; Reset Held Item to Nothing
  (`PrimitiveComponent.SetCollisionEnabled` _key "QueryAndPhysics")
  (`PrimitiveComponent.SetSimulatePhysics` _key true)
  (`PrimitiveComponent.AddImpulse` _key (* (`SceneComponent.GetForwardVector` _key) 1000.0) "None" false))

(event `/Game/Developer/Interaction/BPI_Item.Use`
  (bind _key (`self.Key`))
  (bind _returnvalue (`SceneComponent.K2_GetComponentLocation` _key))
  ; Use Held Item to open door
  (`KismetSystemLibrary.Delay` 0.2)
  (bind _outhit (`KismetSystemLibrary.LineTraceSingle` :`Start` _returnvalue :`End` (+ _returnvalue (* (`SceneComponent.GetForwardVector` _key) 300.0)) :`TraceChannel` "TraceTypeQuery1" :`DrawDebugType` "ForDuration"))
  (bind _asbp_doorrr (cast `/Game/Developer/Doors_And_Keys/BP_Doorrr` (`.HitActor` (`GameplayStatics.BreakHitResult` _outhit))))
  (`/Game/Developer/BPC/BPC_Interact.TrytoDrop` (`self.Owner_0`))
  (`/Game/Developer/Doors_And_Keys/BP_Doorrr.Open Door` _asbp_doorrr)
  (`self.K2_DestroyActor` self))

(event `/Game/Developer/Interaction/BPI_Item.AlternateUse`)

(event `/Game/Developer/BluePrints/SavingAndLoading/BPI_Activatable.Activate`
  (`self.K2_DestroyActor`))

(fn `PickUp`
  (params (Owner :type "/Game/Developer/BPC/BPC_Interact Object Reference"))
  (returns (`Item Type` :type "/Game/Developer/BluePrints/E_item Enum"))
  (bind _customeplayer (`self.CustomePlayer`))
  (bind _keysobtained (`/Game/Developer/BluePrints/BP_CustomFirstPersonCharacter.KeysObtained` _customeplayer))
  (set `self.Owner_0` Owner)
  (`GameplayStatics.PlaySoundAtLocation` "/Game/Developer/Audio/DoorsAndKeys/SQ_KeyJingling_Cue.SQ_KeyJingling_Cue" (`SceneComponent.RelativeLocation` (`self.Key`)) (struct) 1.0 1.0 0.0 null null null null)
  (`KismetSystemLibrary.PrintString` "You have touched the key")
  (set `/Game/Developer/BluePrints/BP_CustomFirstPersonCharacter.KeysObtained` (+ _keysobtained 1) _customeplayer)
  (`KismetSystemLibrary.PrintString` (`KismetStringLibrary.Concat_StrStr` "The Player has" (`KismetStringLibrary.Conv_IntToString` _keysobtained) "key(s)."))
  (`PrimitiveComponent.SetCollisionEnabled` (`self.Key`) "NoCollision")
  ; We have been picked up so don't exist in the next load.
  (bind _asgm_save_load (cast `/Game/Developer/BluePrints/SavingAndLoading/GM_SaveLoad` (`GameplayStatics.GetGameMode`)))
  (`/Game/Developer/BluePrints/SavingAndLoading/SG_LevelState.AddActor` (`/Game/Developer/BluePrints/SavingAndLoading/GM_SaveLoad.LevelState` _asgm_save_load) self)
  (return (`self.ItemType`)))

(fn `UserConstructionScript`)