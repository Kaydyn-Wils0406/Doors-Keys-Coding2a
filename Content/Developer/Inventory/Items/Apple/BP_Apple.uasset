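; BP_Apple is an apple item actor that a character or other owner can pick up and drop.
; PickUp stores the owner, disables collision on the Sphere component and returns the item type.
; Drop clears the owner's HeldItem, re-enables collision and physics on the Sphere, then throws it with an impulse along its forward vector.
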(event `/Game/Developer/Interaction/BPI_Item.Drop`
  (bind _sphere (`self.Sphere`))
  (set `/Game/Developer/Interaction/BPC_Interact.HeldItem` null (`self.Owner_0`)) ; Reset Held Item to Nothing
  (`PrimitiveComponent.SetCollisionEnabled` _sphere "QueryAndPhysics")
  (`PrimitiveComponent.SetSimulatePhysics` _sphere true)
  (`PrimitiveComponent.AddImpulse` _sphere (* (`SceneComponent.GetForwardVector` _sphere) 1000.0) "None" false))

(fn `PickUp`
  (params (Owner :type "/Game/Developer/Interaction/BPC_Interact Object Reference"))
  (returns (`Item Type` :type "/Game/Developer/BluePrints/E_item Enum"))
  (set `self.Owner_0` Owner)
  (`PrimitiveComponent.SetCollisionEnabled` (`self.Sphere`) "NoCollision")
  (return (`self.ItemType`)))

(fn `UserConstructionScript`)