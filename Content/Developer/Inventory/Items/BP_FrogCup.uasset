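; BP_FrogCup is a holdable inventory item, a cup that can be drunk from, swung as if to hit, or dropped.
; Use and AlternateUse wait briefly, then animate the mesh through timelines; drinking reverses after a delay, guarded by HasBeenUsed.
; PickUp stores the owner, disables collision and returns the item type.
; Drop clears the owner's held item, restores physics and throws the cup along its forward vector.
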(event `/Game/Developer/Interaction/BPI_Item.AlternateUse`
  (`KismetSystemLibrary.Delay` 0.2)
  (bind (_direction _hit) (`Timeline|UseToHit` :!via `PlayFromStart`)
    (:`Update`
      (`SceneComponent.K2_SetRelativeLocation` (`self.StaticMesh`) (`KismetMathLibrary.VLerp` (0.0 0.0 0.0) (20.0 0.0 50.0) _hit) false false))))

(event `/Game/Developer/Interaction/BPI_Item.Use`
  ; Drink
  (`KismetSystemLibrary.Delay` 0.2)
  (set `self.bHasBeenUsed` true)
  (bind (_direction _translation _rotation) (`Timeline|Drink` :!via `PlayFromStart` :!label _label)
    (:`Update`
      (`SceneComponent.K2_SetRelativeLocationAndRotation` (`self.StaticMesh`) (`KismetMathLibrary.VLerp` (0.0 0.0 0.0) (-10.0 -25.0 10.0) _translation) (`KismetMathLibrary.RLerp` (struct) (struct :`Yaw` -90.0 :`Roll` -30.0) _rotation) false false)
      (`KismetSystemLibrary.Delay` 2.0)
      (`self.GoBackToNormal`))))

(event `GoBackToNormal`
  ; Drink
  (if (`self.bHasBeenUsed`)
    (set `self.bHasBeenUsed` false)
    (goto _label :!via `ReverseFromEnd`)))

(event `/Game/Developer/Interaction/BPI_Item.Drop`
  (set `/Game/Developer/BPC/BPC_Interact.HeldItem` null (`self.Owner_0`))
  (`PrimitiveComponent.SetCollisionEnabled` (`self.StaticMesh`) "QueryAndPhysics")
  (`PrimitiveComponent.SetSimulatePhysics` (`self.StaticMesh`) true)
  (`PrimitiveComponent.AddImpulse` (`self.StaticMesh`) (* (`SceneComponent.GetForwardVector` (`self.StaticMesh`)) 500.0) "None" false))

(fn `PickUp`
  (params (Owner :type "/Game/Developer/BPC/BPC_Interact Object Reference"))
  (returns (`Item Type` :type "/Game/Developer/BluePrints/E_item Enum"))
  (set `self.Owner_0` Owner)
  (`PrimitiveComponent.SetCollisionEnabled` (`self.StaticMesh`) "NoCollision")
  (return (`self.ItemType`)))

(fn `UserConstructionScript`)