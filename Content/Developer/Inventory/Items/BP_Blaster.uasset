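; BP_Blaster is a blaster inventory item that can be picked up and dropped by an owner.
; PickUp stores the owner, disables collision on the Blaster component and returns the item type.
; Drop clears the owner's HeldItem, restores collision and physics, then throws the blaster along its forward vector with an impulse.
; The Use event is an empty stub, so no firing behavior exists yet.
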(event `self.ReceiveBeginPlay`)

(event `/Game/Developer/Interaction/BPI_Item.Drop`
  (bind _blaster (`self.Blaster`))
  (set `/Game/Developer/Interaction/BPC_Interact.HeldItem` null (`self.Owner_0`)) ; Reset Held Item to Nothing
  (`PrimitiveComponent.SetCollisionEnabled` _blaster "QueryAndPhysics")
  (`PrimitiveComponent.SetSimulatePhysics` _blaster true)
  (`PrimitiveComponent.AddImpulse` _blaster (* (`SceneComponent.GetForwardVector` _blaster) 1000.0) "None" false))

(event `/Game/Developer/Interaction/BPI_Item.Use`)

(fn `PickUp`
  (params (Owner :type "/Game/Developer/Interaction/BPC_Interact Object Reference"))
  (returns (`Item Type` :type "/Game/Developer/BluePrints/E_item Enum"))
  (set `self.Owner_0` Owner)
  (`PrimitiveComponent.SetCollisionEnabled` (`self.Blaster`) "NoCollision")
  (return (`self.ItemType`)))

(fn `UserConstructionScript`)