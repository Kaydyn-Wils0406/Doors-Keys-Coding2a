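; BP_Blaster is a held inventory weapon that can be picked up, dropped and fired.
; PickUp stores the owner, disables mesh collision and returns the item type.
; Drop clears the owner's held item, restores collision and physics, and throws the blaster forward with an impulse.
; Use spawns a BP_Bullet at the Bulletspawn point and launches it forward with a velocity-change impulse on its sphere.
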(event `self.ReceiveBeginPlay`)

(event `/Game/Developer/Interaction/BPI_Item.Drop`
  (bind _blaster (`self.Blaster`))
  (set `/Game/Developer/Interaction/BPC_Interact.HeldItem` null (`self.Owner_0`)) ; Reset Held Item to Nothing
  (`PrimitiveComponent.SetCollisionEnabled` _blaster "QueryAndPhysics")
  (`PrimitiveComponent.SetSimulatePhysics` _blaster true)
  (`PrimitiveComponent.AddImpulse` _blaster (* (`SceneComponent.GetForwardVector` _blaster) 1000.0) "None" false))

(event `/Game/Developer/Interaction/BPI_Item.Use`
  (`self.FireProjectile`))

(event `FireProjectile`
  (bind _bulletspawn (`self.bulletspawn`))
  (bind _returnvalue (`|SpawnActorFromClass` "/Game/Developer/Inventory/Items/Blaster/BP_Bullet.BP_Bullet_C" (`SceneComponent.K2_GetComponentToWorld` _bulletspawn) "Undefined" "MultiplyWithRoot" null null))
  (`PrimitiveComponent.AddImpulse` (`/Game/Developer/Inventory/Items/Blaster/BP_Bullet.Sphere` _returnvalue) (* (`SceneComponent.GetForwardVector` _bulletspawn) 30000.0) "None" true))

(fn `PickUp`
  (params (Owner :type "/Game/Developer/Interaction/BPC_Interact Object Reference"))
  (returns (`Item Type` :type "/Game/Developer/BluePrints/E_item Enum"))
  (set `self.Owner_0` Owner)
  (`PrimitiveComponent.SetCollisionEnabled` (`self.Blaster`) "NoCollision")
  (return (`self.ItemType`)))

(fn `UserConstructionScript`)