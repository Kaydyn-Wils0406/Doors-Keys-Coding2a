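; BPC_Inventory is an inventory component that stores each slot as an item enum in an array.
; GetSlot resolves a slot's enum to its details through GetItemDetails, which scans every DT_Items row for the matching enum.
; SetSlot and SetEnumArray write one slot or the whole array, then fire OnSlotUpdated or OnRefreshGrid so listeners can react.
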(fn `GetItemDetails`
  (params (`Requested Item` :type "/Game/Developer/BluePrints/E_item Enum" :default "NewEnumerator0"))
  (returns (`Item Details` :type "/Game/Developer/Inventory/S_Item Structure"))
  (bind _outrownames (`DataTableFunctionLibrary.GetDataTableRowNames` "/Game/Developer/BluePrints/DataTables/DT_Items.DT_Items"))
  (for _array_element _outrownames
    (bind _returnvalue (`|GetDataTableRow` "/Game/Developer/BluePrints/DataTables/DT_Items.DT_Items" _array_element)
      (:`then`
        (if (`|EnumEquality` (`.Enum_18_F1B54522430B8E96DB230AAE1D3993CA` (break `/Game/Developer/Inventory/S_Item` _returnvalue)) `Requested Item`)
          (return _returnvalue) ; Return the data table row that was requested
        )))))

(fn `GetSlot`
  (params (RequestedSlot :type Integer))
  (returns (`Item Details` :type "/Game/Developer/Inventory/S_Item Structure"))
  (bind _item_details (`self.GetItemDetails` (`|GetArrayItem` (`self.EnumInventory`) RequestedSlot)))
  (return _item_details))

(fn `SetEnumArray`
  (params (EnumInventory :type "Array of /Game/Developer/BluePrints/E_item Enum"))
  (set `self.EnumInventory` EnumInventory)
  (`self.OnRefreshGrid`))

(fn `SetSlot`
  (params (Item :type "/Game/Developer/BluePrints/E_item Enum" :default "NewEnumerator0") (`Slot Index` :type Integer))
  (`KismetArrayLibrary.Array_Set` (`self.EnumInventory`) `Slot Index` Item)
  (`self.OnSlotUpdated` `Slot Index`))