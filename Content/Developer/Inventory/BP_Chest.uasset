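; Inventory chest actor that opens when the first-person character enters its sphere and closes when they leave.
; An Open timeline, played or reversed, drives the hinge rotation; finishing an opening shows the W_ChestMenu widget created at BeginPlay and the player's inventory.
; Player overlap also adds the chest's BPCInventory to GM_SaveLoad's LevelState, and LoadSavedInventory restores a saved inventory onto that component.
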(event `self.ReceiveBeginPlay`
  (`|ExecutionSequence`
    (:`then_0`
      (bind _returnvalue (`|CreateWidget` "/Game/Developer/UI/W_ChestMenu.W_ChestMenu_C" null 0 (`self.BPC_Inventory`)))
      (set `self.ChestMenuWidget` _returnvalue))))

(event `Load Saved Inventory`
  (params (EnumInventory :type "Array of /Game/Developer/BluePrints/E_item Enum"))
  (set `/Game/Developer/Inventory/BPC_Inventory.EnumInventory` EnumInventory (`self.BPC_Inventory`)) ; Replace current INV\nwith saved INV
)

(event `self.sphere_0.OnComponentBeginOverlap`
  (params (OverlappedComponent :type "PrimitiveComponent Object Reference") (OtherActor :type "Actor Object Reference") (OtherComp :type "PrimitiveComponent Object Reference") (OtherBodyIndex :type Integer) (bFromSweep :type Boolean) (SweepResult :type "HitResult Structure (by ref)"))
  (bind _asbp_custom_first_person_character (cast `/Game/Developer/BluePrints/BP_CustomFirstPersonCharacter` OtherActor))
  (`self.OpenChest` false)
  (bind _asgm_save_load (cast `/Game/Developer/BluePrints/SavingAndLoading/GM_SaveLoad` (`GameplayStatics.GetGameMode`)))
  (`/Game/Developer/BluePrints/SavingAndLoading/SG_LevelState.Add Inventory` (`/Game/Developer/BluePrints/SavingAndLoading/GM_SaveLoad.LevelState` _asgm_save_load) (`self.BPC_Inventory`)))

(event `self.sphere_0.OnComponentEndOverlap`
  (params (OverlappedComponent :type "PrimitiveComponent Object Reference") (OtherActor :type "Actor Object Reference") (OtherComp :type "PrimitiveComponent Object Reference") (OtherBodyIndex :type Integer))
  (cast `/Game/Developer/BluePrints/BP_CustomFirstPersonCharacter` OtherActor)
  (`self.OpenChest` true))

(event `OpenChest`
  (params (Reverse :type Boolean))
  ; Hinge Movement
  (if Reverse
    (bind (_direction _open) (`Timeline|Open` :!via `Reverse` :!label _label)
      (:`Update`
        (`SceneComponent.K2_SetWorldRotation` (`self.RealHingeA`) (`KismetMathLibrary.MakeRotator` (`KismetMathLibrary.Lerp` _open 0.0 70.0)) false false))
      (:`Finished`
        (if (not Reverse)
          (`KismetSystemLibrary.PrintText` "Opening Chest")
          ; Showing Inventory
          (`UserWidget.AddToViewport` (`self.ChestMenuWidget`) 0)
          (`/Game/Developer/BluePrints/BP_CustomFirstPersonCharacter.ShowInventory` (stale `self.sphere_0.OnComponentBeginOverlap` _asbp_custom_first_person_character)))))
    (else
      (goto _label))))

(fn `UserConstructionScript`)