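; Checkpoint actor that saves the player's progress when they overlap it.
; On BeginPlay it caches the GM_SaveLoad game mode.
; When a BP_CustomFirstPersonCharacter begins overlap, it passes that character's belt inventory, backpack inventory and transform to the game mode's Save function, then prints an activation message.
; It has no one-shot guard, so each new overlap calls Save again.
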(event `self.ReceiveBeginPlay`
  (bind _asgm_save_load (cast `/Game/Developer/BluePrints/SavingAndLoading/GM_SaveLoad` (`GameplayStatics.GetGameMode`)))
  (set `self.As GM Save Load` _asgm_save_load))

(event `self.ReceiveActorBeginOverlap`
  (params (OtherActor :type "Actor Object Reference"))
  (bind _asbp_custom_first_person_character (cast `/Game/Developer/BluePrints/BP_CustomFirstPersonCharacter` OtherActor)) ; When player overlaps, calls the save\nfunction on the SaveLoad.
  (`/Game/Developer/BluePrints/SavingAndLoading/GM_SaveLoad.Save` (`self.As GM Save Load`) (`/Game/Developer/Inventory/BPC_Inventory.EnumInventory` (`/Game/Developer/BluePrints/BP_CustomFirstPersonCharacter.BPC_BeltInv` _asbp_custom_first_person_character)) (`/Game/Developer/Inventory/BPC_Inventory.EnumInventory` (`/Game/Developer/BluePrints/BP_CustomFirstPersonCharacter.BPC_BackpackInv` _asbp_custom_first_person_character)) (`self.GetTransform` _asbp_custom_first_person_character))
  (`KismetSystemLibrary.PrintString` "Checkpoint Activated"))

(fn `UserConstructionScript`)