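; GM_SaveLoad manages saving, loading and deleting of player inventory and per-level state.
; BeginPlay loads existing saves or creates SG_Player and SG_LevelState objects, the latter stored in a slot prefixed with the level name.
; Save writes both; Load refills the character's belt and backpack, activates actors and respawns added ones, restoring player transform inside that spawn loop.
; Deleting level state reopens the level; DeleteSave also clears the player slot.
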(event `self.ReceiveBeginPlay`
  (`KismetSystemLibrary.PrintText` "Starting GM_SaveLoad" true true (struct :`R` 1.0 :`B` 0.853154 :`A` 1.0) 5.0)
  (`|ExecutionSequence`
    (:`then_0`
      (bind _returnvalue (`GameplayStatics.DoesSaveGameExist` (`self.Slot Name`)))
      (if _returnvalue
        (`KismetSystemLibrary.Delay` 0.2)
        (`self.Load`)
        (`KismetSystemLibrary.PrintText` "called load")
        (else
          (bind _returnvalue_2 (`GameplayStatics.CreateSaveGameObject` "/Game/Developer/BluePrints/SavingAndLoading/SG_Player.SG_Player_C"))
          (set `self.PlayerSave` _returnvalue_2)
          (`KismetSystemLibrary.PrintText` "created sace game"))))
    (:`then_1`
      (bind _returnvalue_3 (`GameplayStatics.GetCurrentLevelName` true))
      (bind _returnvalue_4 (`GameplayStatics.DoesSaveGameExist` (`KismetStringLibrary.Concat_StrStr` _returnvalue_3 "_" (`self.Slot Name`))))
      (if _returnvalue_4
        (`self.Load`)
        (else
          (bind _returnvalue_5 (`GameplayStatics.CreateSaveGameObject` "/Game/Developer/BluePrints/SavingAndLoading/SG_LevelState.SG_LevelState_C"))
          (set `self.LevelState` _returnvalue_5))))))

(fn `DeleteLevelSave`
  (bind _returnvalue (`GameplayStatics.GetCurrentLevelName` true))
  (`GameplayStatics.DeleteGameInSlot` (`KismetStringLibrary.Concat_StrStr` _returnvalue "_" (`self.Slot Name`)))
  (`GameplayStatics.OpenLevel` (`KismetStringLibrary.Conv_StringToName` _returnvalue)))

(fn `DeleteSave`
  (`GameplayStatics.DeleteGameInSlot` (`self.Slot Name`))
  (`self.DeleteLevelSave`))

(fn `Load`
  (bind _player_transform (`/Game/Developer/BluePrints/SavingAndLoading/SG_LevelState.Player Transform` (`self.LevelState`)))
  (bind _actorsadded (`/Game/Developer/BluePrints/SavingAndLoading/SG_LevelState.ActorsAdded` (`self.LevelState`)))
  (`|ExecutionSequence`
    (:`then_0`
      ; Comment
      (bind _returnvalue (`GameplayStatics.LoadGameFromSlot` (`self.Slot Name`))) ; Load from file
      (bind _assg_player (cast `/Game/Developer/BluePrints/SavingAndLoading/SG_Player` _returnvalue)) ; cast to specific SG_player
      (set `self.PlayerSave` _assg_player) ; store this as a variable
      (bind _asbp_custom_first_person_character (cast `/Game/Developer/BluePrints/BP_CustomFirstPersonCharacter` (`GameplayStatics.GetPlayerCharacter` 0)) ; get a reference to player
        (:`then`
          (`/Game/Developer/Inventory/BPC_Inventory.SetEnumArray` (`/Game/Developer/BluePrints/BP_CustomFirstPersonCharacter.BPC_BeltInv` _asbp_custom_first_person_character) (`/Game/Developer/BluePrints/SavingAndLoading/SG_Player.Belt` (`self.PlayerSave`)))
          (`/Game/Developer/Inventory/BPC_Inventory.SetEnumArray` (`/Game/Developer/BluePrints/BP_CustomFirstPersonCharacter.BPC_BackpackInv` _asbp_custom_first_person_character) (`/Game/Developer/BluePrints/SavingAndLoading/SG_Player.PlayerInv` (`self.PlayerSave`)))
          (`KismetSystemLibrary.PrintText` "Inventories Updated"))
        (:`CastFailed`
          (`KismetSystemLibrary.PrintString` "Not the Player"))))
    (:`then_1`
      ; Load Game State
      (bind _returnvalue_2 (`GameplayStatics.GetCurrentLevelName` true))
      (bind _returnvalue_3 (`GameplayStatics.LoadGameFromSlot` (`KismetStringLibrary.Concat_StrStr` _returnvalue_2 "_" (`self.Slot Name`))))
      (bind _assg_level_state (cast `/Game/Developer/BluePrints/SavingAndLoading/SG_LevelState` _returnvalue_3))
      (bind _output_get (set `self.LevelState` _assg_level_state))
      (`/Game/Developer/BluePrints/SavingAndLoading/SG_LevelState.ActivateActors` _output_get)
      (bind _keys (`BlueprintMapLibrary.Map_Keys` _actorsadded))
      (for _array_element _keys
        (`|SpawnActorFromClass` (`|ConvertAsset` _array_element) (`BlueprintMapLibrary.Map_Find` _actorsadded _array_element) "Undefined" "MultiplyWithRoot" null null)
        (bind _asbp_custom_first_person_character_2 (cast `/Game/Developer/BluePrints/BP_CustomFirstPersonCharacter` (`GameplayStatics.GetPlayerCharacter` 0)))
        (`/Game/Developer/BluePrints/BP_CustomFirstPersonCharacter.Load Transform` _asbp_custom_first_person_character_2 _player_transform)
        ;; Should Go on Character
        (`Controller.SetControlRotation` (`GameplayStatics.GetPlayerController` 0) (.rotation _player_transform))))))

(fn `Save`
  (params (Belt :type "Array of /Game/Developer/BluePrints/E_item Enum") (PlayerInv :type "Array of /Game/Developer/BluePrints/E_item Enum") (Location :type "Transform Structure"))
  (bind _playersave (`self.PlayerSave`))
  ; Saving Player Inventories
  (`|ExecutionSequence`
    (:`then_0`
      (set `/Game/Developer/BluePrints/SavingAndLoading/SG_Player.Belt` Belt _playersave)
      (set `/Game/Developer/BluePrints/SavingAndLoading/SG_Player.PlayerInv` PlayerInv _playersave)
      (`GameplayStatics.SaveGameToSlot` (`self.PlayerSave`) (`self.Slot Name`)) ; Save Game to file
    )
    (:`then_1`
      ; Saving Level State
      (set `/Game/Developer/BluePrints/SavingAndLoading/SG_LevelState.Player Transform` Location (`self.LevelState`))
      (bind _returnvalue (`GameplayStatics.GetCurrentLevelName` true))
      (`GameplayStatics.SaveGameToSlot` (`self.LevelState`) (`KismetStringLibrary.Concat_StrStr` _returnvalue "_" (`self.Slot Name`))) ; Save Game to file
    )))

(fn `UserConstructionScript`)