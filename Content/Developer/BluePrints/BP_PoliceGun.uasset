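; BP_PoliceGun is a holdable police gun item with pick up, drop, use and alternate use events.
; Pickup disables collision; drop clears the owner's HeldItem, re-enables collision and physics, and tosses the gun forward.
; Use and AlternateUse animate aim-and-shoot and melee swing poses through timeline-driven relative transform lerps, then return after delays.
; Both actions are purely visual apart from debug prints, with no projectile, trace or damage logic.
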(event `/Game/Developer/Interaction/BPI_Item.PickUp`
  (params (Owner :type "/Game/Developer/Interaction/BPC_Interact Object Reference"))
  ; PickUp and Drop
  (`PrimitiveComponent.SetCollisionEnabled` (`self.PoliceGun`) "NoCollision"))

(event `/Game/Developer/Interaction/BPI_Item.Drop`
  (bind _policegun (`self.PoliceGun`))
  ; PickUp and Drop
  (set `/Game/Developer/Interaction/BPC_Interact.HeldItem` null (stale `/Game/Developer/Interaction/BPI_Item.PickUp` Owner))
  (`PrimitiveComponent.SetCollisionEnabled` _policegun "QueryAndPhysics")
  (`PrimitiveComponent.SetSimulatePhysics` _policegun true)
  (`PrimitiveComponent.AddImpulse` _policegun (* (`SceneComponent.GetForwardVector` _policegun) 500.0) "None" false))

(event `/Game/Developer/Interaction/BPI_Item.Use`
  ; Use
  (`KismetSystemLibrary.PrintString` "Used Gun")
  (`KismetSystemLibrary.Delay` 0.2)
  (set `self.bHasBeenUsed` true)
  (bind (_direction _shooting _aim) (`Timeline|Shoot` :!via `PlayFromStart` :!label _label)
    (:`Update`
      (`SceneComponent.K2_SetRelativeLocationAndRotation` (`self.PoliceGun`) (`KismetMathLibrary.VLerp` (0.0 0.0 0.0) (0.0 -15.0 30.0) _aim) (`KismetMathLibrary.RLerp` (struct) (struct :`Pitch` 60.0) _shooting) false false)
      (`KismetSystemLibrary.Delay` 1.0)
      (`self.BackToStart`))))

(event `BackToStart`
  ; Use
  (if (`self.bHasBeenUsed`)
    (set `self.bHasBeenUsed` false)
    (goto _label :!via `ReverseFromEnd`)))

(event `/Game/Developer/Interaction/BPI_Item.AlternateUse`
  (`KismetSystemLibrary.PrintString` "Alternate Used Gun")
  (`KismetSystemLibrary.Delay` 0.2)
  (bind (_direction _turn _swing) (`Timeline|HitWithGun` :!via `PlayFromStart`)
    (:`Update`
      (bind _returnvalue (`KismetMathLibrary.VLerp` (0.0 0.0 20.0) (0.0 -45.0 20.0) _turn))
      (bind _returnvalue_2 (`KismetMathLibrary.RLerp` (struct) (struct :`Yaw` -50.0 :`Roll` -90.0) _turn))
      (`SceneComponent.K2_SetRelativeLocationAndRotation` (`self.PoliceGun`) _returnvalue _returnvalue_2 false false)
      (bind _returnvalue_3 (`KismetMathLibrary.VLerp` _returnvalue (20.0 15.0 20.0) _swing))
      (bind _returnvalue_4 (`KismetMathLibrary.RLerp` _returnvalue_2 (struct :`Yaw` 90.0 :`Roll` -90.0) _swing))
      (`SceneComponent.K2_SetRelativeLocationAndRotation` (`self.PoliceGun`) _returnvalue_3 _returnvalue_4 false false)
      (`KismetSystemLibrary.Delay` 1.0)
      (bind (_direction_2 _holder) (`Timeline|Back To Hold` :!via `PlayFromStart`)
        (:`Update`
          (`SceneComponent.K2_SetRelativeLocationAndRotation` (`self.PoliceGun`) (`KismetMathLibrary.VLerp` _returnvalue_3 (0.0 0.0 0.0) _holder) (`KismetMathLibrary.RLerp` _returnvalue_4 (struct) _holder) false false))))))

(fn `NewFunction`)

(fn `UserConstructionScript`)