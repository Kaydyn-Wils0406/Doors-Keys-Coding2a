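; AI controller shared by security cameras and turrets that reacts to what its AI Perception senses.
; On possess it caches the pawn as either a BP_SecurityCamera or a BP_Turret.
; Perception updates skip actors tagged AI, print a debug message, and pass sight stimuli, identified by sense class display name, to HandleSight.
; HandleSight forwards target and detection state to the possessed camera or turret, plus stimulus location for cameras.
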(event `self.ReceivePossess`
  (params (PossessedPawn :type "Pawn Object Reference"))
  (bind _asbp_security_camera (cast `/Game/Developer/BluePrints/AI/BP_SecurityCamera` PossessedPawn)
    (:`then`
      (set `self.SecurityCamera` _asbp_security_camera))
    (:`CastFailed`
      (bind _asbp_turret (cast `/Game/Developer/BluePrints/AI/BP_Turret` PossessedPawn))
      (set `self.As BP Turret` _asbp_turret))))

(event `self.AIPerception.OnTargetPerceptionUpdated`
  (params (Actor :type "Actor Object Reference") (Stimulus :type "AIStimulus Structure"))
  (bind (_age _expirationage _strength _stimuluslocation _receiverlocation _tag _bsuccessfullysensed) (break `AIStimulus` Stimulus))
  (if (not (`self.ActorHasTag` Actor "AI"))
    (bind _returnvalue (`AIPerceptionSystem.GetSenseClassForStimulus` Stimulus))
    (bind _returnvalue_2 (`KismetSystemLibrary.GetClassDisplayName` _returnvalue))
    (`KismetSystemLibrary.PrintText` (`|FormatText` "Sensed: {actor} with {name} and the tag {tag}." Actor _returnvalue_2 _tag))
    (switch `name` _tag
      (:`Default`
        (switch `string` _returnvalue_2
          (:`AISense_Sight`
            (`self.HandleSight` _bsuccessfullysensed _stimuluslocation Actor))))
      (:`AI`
        (`KismetSystemLibrary.PrintText` "Hello AI Buddy")))))

(fn `HandleSight`
  (params (SuccessfullySensed1 :type Boolean) (StimulusLocation1 :type "Vector Structure") (Target1 :type "Actor Object Reference"))
  (bind _securitycamera (`self.SecurityCamera`)
    (:`then`
      (`/Game/Developer/BluePrints/AI/BP_SecurityCamera.HandleSight` _securitycamera SuccessfullySensed1 StimulusLocation1 Target1))
    (:`else`
      (bind _as_bp_turret (`self.As BP Turret`)
        (:`then`
          (`/Game/Developer/BluePrints/AI/BP_Turret.Handle Sight` _as_bp_turret Target1 SuccessfullySensed1))
        (:`else`)))))

(fn `UserConstructionScript`)