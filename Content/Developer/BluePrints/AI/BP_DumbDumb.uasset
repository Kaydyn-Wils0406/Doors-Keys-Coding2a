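; BP_DumbDumb is a simple AI pawn that investigates a security alarm location and then returns to where it started.
; It records its starting location on BeginPlay.
; CheckOutSecurityAlarm prints a debug message and uses AIMoveTo to walk to the given location.
; Whether the move succeeds or fails, it waits briefly, then GoHome moves it back to the stored start location.
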(event `self.ReceiveBeginPlay`
  (set `self.StartLocation` (`self.K2_GetActorLocation`)))

(event `CheckOutSecurityAlarm`
  (params (Location :type "Vector Structure"))
  (`KismetSystemLibrary.PrintText` "DumbDumb is moving toward the Stimulus Location.")
  (`|AIMoveTo` self Location null
    (:`OnSuccess`
      _)
    (:`OnFail`
      _))
  (`KismetSystemLibrary.Delay` 2.0)
  (`self.GoHome`))

(event `GoHome`
  (`|AIMoveTo` self (`self.StartLocation`) null))

(fn `UserConstructionScript`)