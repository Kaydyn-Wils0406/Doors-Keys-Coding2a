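; BP_SecurityCamera is an AI security camera that raises an alarm when it senses a target by sight.
; HandleSight branches on the sensing result, switching the mesh between red and green materials with a matching sound and debug text.
; On detection, it finds every BP_DumbDumb actor in the level and calls CheckOutSecurityAlarm on each with the stimulus location.
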(fn `HandleSight`
  (params (SuccessfullySensed :type Boolean) (StimulusLocation :type "Vector Structure") (Target :type "Actor Object Reference"))
  (bind _returnvalue (`self.K2_GetActorLocation`))
  (bind _staticmesh (`self.StaticMesh`))
  (if SuccessfullySensed
    (`KismetSystemLibrary.PrintText` "You are being seen.")
    (`PrimitiveComponent.SetMaterial` _staticmesh 0 "/AnimationSharing/AnimSharingRed.AnimSharingRed")
    (`GameplayStatics.PlaySoundAtLocation` "/Engine/EditorSounds/Notifications/CompileFailed.CompileFailed" _returnvalue (struct) 1.0 1.0 0.0 "/Game/Developer/Audio/Attenuation.Attenuation" null null null)
    (bind _outactors (`GameplayStatics.GetAllActorsOfClass` "/Game/Developer/BluePrints/AI/BP_DumbDumb.BP_DumbDumb_C"))
    (for _array_element _outactors
      (`/Game/Developer/BluePrints/AI/BP_DumbDumb.CheckOutSecurityAlarm` _array_element StimulusLocation))
    (else
      (`KismetSystemLibrary.PrintText` "You are not being seen.")
      (`PrimitiveComponent.SetMaterial` _staticmesh 0 "/AnimationSharing/AnimSharingGreen.AnimSharingGreen")
      (`GameplayStatics.PlaySoundAtLocation` "/Engine/EditorSounds/Notifications/CompileSuccess.CompileSuccess" _returnvalue (struct) 1.0 1.0 0.0 "/Game/Developer/Audio/Attenuation.Attenuation" null null null))))

(fn `UserConstructionScript`)