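; BPC_Stats is a component that holds a stats struct with health, mana, stamina, gold, experience and a saved location.
; Tick calls DebugStats to print the current values as on-screen text each frame, with the frame's delta time as display duration.
; GetCanSprint reports whether any stamina remains, and Sprinting subtracts a given amount of stamina without clamping.
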(event `self.ReceiveTick`
  (params (DeltaSeconds :type "Float (single-precision)"))
  (`self.Debug Stats` DeltaSeconds))

(event `Debug Stats`
  (params (Duration :type "Float (double-precision)"))
  (bind (_health _mana _stamina _savedlocation _gold _experience) (break `/Game/Developer/BluePrints/S_Stats` (`self.Stats`)))
  (`KismetSystemLibrary.PrintText` (`|FormatText` "HP: {health}, MP: {mana}, Stam: {stamina}, Gold: {gold}, XP: {experience}" _health _mana _stamina _gold _experience) true true (struct :`R` 1.0 :`G` 0.353253 :`A` 1.0) Duration))

(fn `GetCanSprint`
  (returns (CanSprint :type Boolean))
  (bind (_stats_health _stats_mana _stats_stamina) (break `/Game/Developer/BluePrints/S_Stats` (`self.Stats`)))
  (return (> _stats_stamina 0.0)))

(fn `Sprinting`
  (params (ReduceStaminaBy :type "Float (double-precision)" :default 2.0))
  (bind (_stats_health _stats_mana _stats_stamina _stats_savedlocation _stats_gold _stats_experience) (break `/Game/Developer/BluePrints/S_Stats` (`self.Stats`)))
  (set `self.Stats` (make `/Game/Developer/BluePrints/S_Stats` _stats_health _stats_mana (- _stats_stamina ReduceStaminaBy) _stats_savedlocation _stats_gold _stats_experience))
  (return))