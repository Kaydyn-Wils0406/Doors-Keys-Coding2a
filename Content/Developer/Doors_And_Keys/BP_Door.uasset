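; BP_Door is a hinged door that swings on a timeline-driven yaw rotation and tracks whether the first-person player is inside its box collision.
; Activate calls OpenDoor with false, which registers the door in the GM_SaveLoad level state, plays an unlocking sound, then runs the timeline after a delay.
; Passing true instead reverses the timeline from its end.
; The overlap flag is only set here, and an older reverse-swing branch is left unconnected.
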(event `self.boxcollision.OnComponentBeginOverlap`
  (params (OverlappedComponent :type "PrimitiveComponent Object Reference") (OtherActor :type "Actor Object Reference") (OtherComp :type "PrimitiveComponent Object Reference") (OtherBodyIndex :type Integer) (bFromSweep :type Boolean) (SweepResult :type "HitResult Structure (by ref)"))
  (cast `/Game/Developer/BluePrints/BP_CustomFirstPersonCharacter` OtherActor)
  (set `self.bPlayerInCollision` true))

(event `self.boxcollision.OnComponentEndOverlap`
  (params (OverlappedComponent :type "PrimitiveComponent Object Reference") (OtherActor :type "Actor Object Reference") (OtherComp :type "PrimitiveComponent Object Reference") (OtherBodyIndex :type Integer))
  (cast `/Game/Developer/BluePrints/BP_CustomFirstPersonCharacter` OtherActor)
  (set `self.bPlayerInCollision` false))

(event `OpenDoor`
  (params (Open :type Boolean))
  (if Open
    (bind (_direction _movingdoor) (`Timeline|DoorOpen2` :!via `ReverseFromEnd` :!label _label)
      (:`Update`
        (`SceneComponent.K2_SetRelativeRotation` (`self.Door`) (`KismetMathLibrary.MakeRotator` 0.0 0.0 (`KismetMathLibrary.Lerp` 0.0 -45.0 _movingdoor)) false false)))
    (else
      (bind _asgm_save_load (cast `/Game/Developer/BluePrints/SavingAndLoading/GM_SaveLoad` (`GameplayStatics.GetGameMode`)))
      (`/Game/Developer/BluePrints/SavingAndLoading/SG_LevelState.AddActor` (`/Game/Developer/BluePrints/SavingAndLoading/GM_SaveLoad.LevelState` _asgm_save_load) self)
      (`GameplayStatics.PlaySoundAtLocation` "/Game/Developer/Audio/DoorsAndKeys/SQ_UnlockindDoor_Cue.SQ_UnlockindDoor_Cue" (`SceneComponent.RelativeLocation` (`self.Door`)) (struct) 1.0 1.0 0.0 null null null null)
      (`KismetSystemLibrary.Delay` 2.0)
      (goto _label))))

(event `/Game/Developer/BluePrints/SavingAndLoading/BPI_Activatable.Activate`
  (`self.OpenDoor` false))

(fn `UserConstructionScript`)