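; BP_LevelExit is a level exit trigger that saves the player's state and loads another level.
; On BeginPlay it caches the GM_SaveLoad game mode.
; When BP_CustomFirstPersonCharacter overlaps its Box, it passes the belt inventory, backpack inventory and character transform to the game mode's Save function.
; It then prints a checkpoint message and opens the Destination level by object reference.
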(event `self.ReceiveBeginPlay`
  (bind _asgm_save_load (cast `/Game/Developer/BluePrints/SavingAndLoading/GM_SaveLoad` (`GameplayStatics.GetGameMode`)))
  (set `self.Game Mode` _asgm_save_load))

(event `self.Box.OnComponentBeginOverlap`
  (params (OverlappedComponent :type "PrimitiveComponent Object Reference") (OtherActor :type "Actor Object Reference") (OtherComp :type "PrimitiveComponent Object Reference") (OtherBodyIndex :type Integer) (bFromSweep :type Boolean) (SweepResult :type "HitResult Structure (by ref)"))
  (bind _asbp_custom_first_person_character (cast `/Game/Developer/BluePrints/BP_CustomFirstPersonCharacter` OtherActor)) ; When player overlaps, calls the save\nfunction on the SaveLoad.
  (`/Game/Developer/BluePrints/SavingAndLoading/GM_SaveLoad.Save` (`self.Game Mode`) (`/Game/Developer/Inventory/BPC_Inventory.EnumInventory` (`/Game/Developer/BluePrints/BP_CustomFirstPersonCharacter.BPC_BeltInv` _asbp_custom_first_person_character)) (`/Game/Developer/Inventory/BPC_Inventory.EnumInventory` (`/Game/Developer/BluePrints/BP_CustomFirstPersonCharacter.BPC_BackpackInv` _asbp_custom_first_person_character)) (`self.GetTransform` _asbp_custom_first_person_character))
  (`KismetSystemLibrary.PrintString` "Checkpoint Activated")
  (`GameplayStatics.OpenLevelBySoftObjectPtr` (`self.Destination`)))

(fn `UserConstructionScript`)