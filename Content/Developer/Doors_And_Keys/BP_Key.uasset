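; BP_Key is a holdable key item that the first-person player collects and uses on doors.
; PickUp plays a jingle, increments the player's KeysObtained count and disables collision, while Drop re-enables collision and physics with a forward impulse.
; Use waits briefly, then line-traces forward from BoxCollision; hitting a BP_Door clears the owner's held item, calls the player's UseDoor and destroys the key.
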(event `self.ReceiveBeginPlay`
  (bind _asbp_custom_first_person_character (cast `/Game/Developer/BluePrints/BP_CustomFirstPersonCharacter` (`GameplayStatics.GetPlayerCharacter` 0)))
  (set `self.CustomePlayer` _asbp_custom_first_person_character))

(event `/Game/Developer/Interaction/BPI_Item.Drop`
  (bind _key (`self.Key`))
  (set `/Game/Developer/Interaction/BPC_Interact.HeldItem` null (stale `/Game/Developer/Interaction/BPI_Item.PickUp` Owner))
  (`PrimitiveComponent.SetCollisionEnabled` _key "QueryAndPhysics")
  (`PrimitiveComponent.SetSimulatePhysics` _key true)
  (`PrimitiveComponent.AddImpulse` _key (* (`SceneComponent.GetForwardVector` _key) 1000.0) "None" false))

(event `/Game/Developer/Interaction/BPI_Item.PickUp`
  (params (Owner :type "/Game/Developer/Interaction/BPC_Interact Object Reference"))
  (bind _customeplayer (`self.CustomePlayer`))
  (bind _keysobtained (`/Game/Developer/BluePrints/BP_CustomFirstPersonCharacter.KeysObtained` _customeplayer))
  ; Pick Up Key and Count it for Door
  (`GameplayStatics.PlaySoundAtLocation` "/Game/Developer/Audio/DoorsAndKeys/SQ_KeyJingling_Cue.SQ_KeyJingling_Cue" (`SceneComponent.RelativeLocation` (`self.Key`)) (struct) 1.0 1.0 0.0 null null null null)
  (`KismetSystemLibrary.PrintString` "You have touched the key")
  (set `/Game/Developer/BluePrints/BP_CustomFirstPersonCharacter.KeysObtained` (+ _keysobtained 1) _customeplayer)
  (`KismetSystemLibrary.PrintString` (`KismetStringLibrary.Concat_StrStr` "The Player has" (`KismetStringLibrary.Conv_IntToString` _keysobtained) "key(s)."))
  (`PrimitiveComponent.SetCollisionEnabled` (`self.Key`) "NoCollision"))

(event `/Game/Developer/Interaction/BPI_Item.Use`
  (bind _boxcollision (`self.BoxCollision`))
  (bind _returnvalue (`SceneComponent.K2_GetComponentLocation` _boxcollision))
  ; Use Held Item to open door
  (`KismetSystemLibrary.Delay` 0.2)
  (bind _outhit (`KismetSystemLibrary.LineTraceSingle` :`Start` _returnvalue :`End` (+ _returnvalue (* (`SceneComponent.GetForwardVector` _boxcollision) 300.0)) :`TraceChannel` "TraceTypeQuery1" :`DrawDebugType` "ForDuration"))
  (cast `/Game/Developer/Doors_And_Keys/BP_Door` (`.HitActor` (`GameplayStatics.BreakHitResult` _outhit)))
  (set `/Game/Developer/Interaction/BPC_Interact.HeldItem` null (stale `/Game/Developer/Interaction/BPI_Item.PickUp` Owner))
  (`/Game/Developer/BluePrints/BP_CustomFirstPersonCharacter.Use Door` (`self.CustomePlayer`))
  (`self.K2_DestroyActor` self))

(event `/Game/Developer/Interaction/BPI_Item.AlternateUse`)

(event `/Game/Developer/Interaction/BPI_Item.EmptyHandUse`)

(fn `UserConstructionScript`)