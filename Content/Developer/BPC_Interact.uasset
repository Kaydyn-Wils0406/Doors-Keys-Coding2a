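; BPC_Interact is an actor component that lets the first-person character probe what it is looking at, apparently an early interaction prototype.
; On BeginPlay it casts its owner to BP_FirstPersonCharacter and caches that character's camera.
; TryToInteract line-traces on the Visibility channel from the camera forward by LookDistance, draws the debug trace, and prints the hit actor's name and distance.
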(event `self.ReceiveBeginPlay`
  (bind _asbp_first_person_character (cast `/Game/FirstPerson/Blueprints/BP_FirstPersonCharacter` (`self.GetOwner`)))
  (set `self.First Person Camera` (`/Game/FirstPerson/Blueprints/BP_FirstPersonCharacter.FirstPersonCamera` _asbp_first_person_character)))

(event `Try To Interact`
  (bind _first_person_camera (`self.First Person Camera`))
  (bind _returnvalue (`SceneComponent.K2_GetComponentLocation` _first_person_camera))
  (bind (_outhit _returnvalue_2) (`KismetSystemLibrary.LineTraceSingle` :`Start` _returnvalue :`End` (+ _returnvalue (* (`SceneComponent.GetForwardVector` _first_person_camera) (`self.LookDistance`))) :`TraceChannel` "TraceTypeQuery1" :`DrawDebugType` "ForDuration"))
  (if _returnvalue_2
    (bind (_bblockinghit _binitialoverlap _time _distance _location _impactpoint _normal _impactnormal _physmat _hitactor) (`GameplayStatics.BreakHitResult` _outhit))
    (`KismetSystemLibrary.PrintText` (`|FormatText` "I am touching {Name} {distance} cm away!" (`KismetSystemLibrary.GetDisplayName` _hitactor) _distance))))